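; BP_BassicTurret is an enemy turret that tracks and fires missiles at BasicShip pawns it sees.
; When its PawnSensing component spots a ship, the whole actor snaps to face it using a look-at rotation.
; It then spawns a BasicEnemyMissile at ProjectileSpawnLocation, gated by a CanFire flag that a Delay resets as a short cooldown between shots.
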(event OnSeePawn(PawnSensing)
  (params (Pawn :type Pawn%20Object%20Reference))
  (bind _asbasic_ship (Utilities|Casting|CastToBasicShip Pawn))
  (Utilities|FlowControl|Sequence
    (:then_0
      (Transformation|SetActorRotation (Math|Rotator|FindLookatRotation (Transformation|GetActorLocation) (Transformation|GetActorLocation _asbasic_ship))))
    (:then_1
      (if (Variables|Default|GetCanFire)
        (Game|SpawnActorfromClass "/Game/BasicEnemyMissile.BasicEnemyMissile_C" (Transformation|GetWorldTransform (Variables|Default|GetProjectileSpawnLocation)) "AlwaysSpawn" 0 0)
        (Variables|Default|SetCanFire false)
        (Utilities|FlowControl|Delay 1.0)
        (Variables|Default|SetCanFire true)))))

(fn ConstructionScript)